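; BP_InteractableComponent is an Actor Blueprint base for interactables that signal other actors on or off.
; StateOn and StateOff loop over ActorArray and send SwitchOnMessage or SwitchOffMessage to each actor implementing the I_SignalReceiver interface.
; Interacted is an empty stub, and nothing in this Blueprint calls the state functions, leaving the triggering logic outside this class.
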(event EventBeginPlay)

(event Collision|EventActorBeginOverlap
  (params (OtherActor :type Actor%20Object%20Reference)))

(event EventTick
  (params (DeltaSeconds :type Float%20%28single-precision%29)))

(fn ConstructionScript)

(fn Stateon
  (for _array_element (Variables|Default|GetactorArray)
    (if (Utilities|DoesObjectImplementInterface _array_element "/Game/Test/Test_Interface/I_SignalReceiver.I_SignalReceiver_C")
      (Class|ISignalReceiver|Switchon(Message) _array_element))))

(fn StateOff
  (for _array_element (Variables|Default|GetactorArray)
    (if (Utilities|DoesObjectImplementInterface _array_element "/Game/Test/Test_Interface/I_SignalReceiver.I_SignalReceiver_C")
      (Class|ISignalReceiver|SwitchOff(Message) _array_element))))

(fn Interacted)