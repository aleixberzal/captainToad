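; BP_PickableItem is an actor for a crate the player can pick up and throw.
; PickUp casts the player pawn to BP_ThirdPersonCharacter, disables the crate's physics simulation and attaches it to the character's PickPoint, snapping location.
; ThrowOff re-enables physics, detaches the item and applies a fixed impulse along the character capsule's forward vector.
; Both are functions meant to be called externally, as the event graph holds only disabled placeholder events.
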(event EventBeginPlay)

(event Collision|EventActorBeginOverlap
  (params (OtherActor :type Actor%20Object%20Reference)))

(event EventTick
  (params (DeltaSeconds :type Float%20%28single-precision%29)))

(fn ConstructionScript)

(fn PickUp
  (bind _asbp_third_person_character (Utilities|Casting|CastToBP_ThirdPersonCharacter (Game|Player|GetPlayerPawn 0))
    (:then
      (Physics|SetSimulatePhysics (Variables|Default|Getcrate-item) false)
      (Transformation|AttachComponentToComponent (Variables|/Game/ThirdPerson/Blueprints/BP_ThirdPersonCharacter.BP_ThirdPersonCharacter_C|GetpickPoint _asbp_third_person_character) "None" "SnapToTarget" "KeepRelative" "KeepRelative" true))
    (:CastFailed
      (Development|PrintString "cast failed"))))

(fn ThrowOff
  (bind _asbp_third_person_character (Utilities|Casting|CastToBP_ThirdPersonCharacter (Game|Player|GetPlayerPawn 0)))
  (Physics|SetSimulatePhysics (Variables|Default|Getcrate-item) true)
  (Transformation|DetachFromActor "KeepRelative" "KeepRelative" "KeepRelative")
  (Physics|AddImpulse (Variables|Default|Getcrate-item) (* (Math|Vector|GetForwardVector (Variables|/Script/Engine.Character|GetCapsuleComponent _asbp_third_person_character)) 1.5e+04) "None" false))