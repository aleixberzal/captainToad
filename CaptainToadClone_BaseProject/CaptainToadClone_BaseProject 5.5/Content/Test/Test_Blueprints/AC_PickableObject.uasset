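; Pickable-object component that lets an Interact event attach its owning actor to the player, apparently a test box pickup.
; Interact toggles IsBoxPicked and prints the state, calling TeleportObject only when picking up.
; TeleportObject sets the owner's location using only a Z derived from player height plus an offset, then attaches it to the player's root with KeepRelative rules.
; Un-picking only clears the flag, with no detach.
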(event EventBeginPlay)

(event EventTick
  (params (DeltaSeconds :type Float%20%28single-precision%29)))

(event EventInteract
  (if (not (Variables|Default|GetisBoxPicked))
    (Variables|Default|SetisBoxPicked true)
    (Development|PrintString "Pick Box" true true "(R=1.000000,G=0.000000,B=0.022553,A=1.000000)")
    (CallFunction|TeleportObject)
    (else
      (Variables|Default|SetisBoxPicked false)
      (Development|PrintString "Not Pick Box"))))

(fn TeleportObject
  (Transformation|SetActorLocation (Components|GetOwner) (Math|Vector|MakeVector 0.0 0.0 (+ (.z (Transformation|GetActorLocation (Game|GetPlayerCharacter 0))) 275.0)) false true)
  (Transformation|AttachComponentToComponent (Components|GetOwner) (Variables|/Script/Engine.Actor|GetRootComponent (Game|Player|GetPlayerPawn 0)) "None" "KeepRelative" "KeepRelative" "KeepRelative" true))