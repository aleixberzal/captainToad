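; BP_Door is a test door that swings open and closed through its Switchon and SwitchOff events.
; Switchon plays a timeline that sets the yaw of the Doorrotatelarge mesh, and SwitchOff reverses it.
; The Box overlap events are empty, and an older player-overlap rotation is left disconnected.
; An author note says triggering Switchon from a key-and-lock collision does not work, unlike lever or button-driven platforms.
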(event OnComponentBeginOverlap(Box)
  (params (OverlappedComponent :type Primitive%20Component%20Object%20Reference) (OtherActor :type Actor%20Object%20Reference) (OtherComp :type Primitive%20Component%20Object%20Reference) (OtherBodyIndex :type Integer) (bFromSweep :type Boolean) (SweepResult :type Hit%20Result%20Structure%20%28by%20ref%29)))

(event OnComponentEndOverlap(Box)
  (params (OverlappedComponent :type Primitive%20Component%20Object%20Reference) (OtherActor :type Actor%20Object%20Reference) (OtherComp :type Primitive%20Component%20Object%20Reference) (OtherBodyIndex :type Integer)))

(event EventBeginPlay)

(event Collision|EventActorBeginOverlap
  (params (OtherActor :type Actor%20Object%20Reference)))

(event EventTick
  (params (DeltaSeconds :type Float%20%28single-precision%29)))

(event EventSwitchOff
  ;[0.15 0.00619 0 0.5] En principio, al activar el switch on con la colisión de la llave con el lock, debería activarse este evento como lo hace con las plataformas al activar la palanca o el botón pero no funciona y no sé por qué.
  (bind _rotation (Timeline|Timeline Reverse)
    (:Update
      (Transformation|SetRelativeRotation (Variables|Default|Getdoor-rotate-large) (Math|Rotator|MakeRotator 0.0 0.0 _rotation) false false))))

(event EventSwitchon
  ;[0.15 0.00619 0 0.5] En principio, al activar el switch on con la colisión de la llave con el lock, debería activarse este evento como lo hace con las plataformas al activar la palanca o el botón pero no funciona y no sé por qué.
  (bind _rotation (Timeline|Timeline Play)
    (:Update
      (Transformation|SetRelativeRotation (Variables|Default|Getdoor-rotate-large) (Math|Rotator|MakeRotator 0.0 0.0 _rotation) false false))))

(fn ConstructionScript)