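; BP_Lift is a lift actor that travels between a start and end point when switched on or off.
; On BeginPlay it converts the StartPoint and EndPoint offsets to world positions using the root's location.
; Switchon plays the Up timeline, whose track drives a vector lerp that sets the actor's location without sweeping.
; SwitchOff reverses the same timeline to send the lift back.
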(event EventBeginPlay
  (Variables|Default|SetstartPoint (+ (Transformation|GetWorldLocation (Variables|Default|GetDefaultSceneRoot)) (Variables|Default|GetstartPoint)))
  (Variables|Default|SetendPoint (+ (Transformation|GetWorldLocation (Variables|Default|GetDefaultSceneRoot)) (Variables|Default|GetendPoint))))

(event Collision|EventActorBeginOverlap
  (params (OtherActor :type Actor%20Object%20Reference)))

(event EventTick
  (params (DeltaSeconds :type Float%20%28single-precision%29)))

(event EventSwitchon
  (bind _newtrack_0 (Timeline|Up Play)
    (:Update
      (Transformation|SetActorLocation (Math|Vector|Lerp(Vector) (Variables|Default|GetstartPoint) (Variables|Default|GetendPoint) _newtrack_0) false false))))

(event EventSwitchOff
  (bind _newtrack_0 (Timeline|Up Reverse)
    (:Update
      (Transformation|SetActorLocation (Math|Vector|Lerp(Vector) (Variables|Default|GetstartPoint) (Variables|Default|GetendPoint) _newtrack_0) false false))))

(fn ConstructionScript)