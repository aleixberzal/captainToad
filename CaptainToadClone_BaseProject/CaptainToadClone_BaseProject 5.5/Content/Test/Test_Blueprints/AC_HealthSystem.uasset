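; Health component that tracks hit points, shows them on the gameplay HUD and handles player respawn.
; BeginPlay creates the W_GamePlayTest widget without checking whether the owner is the player, then fills health to max.
; RemoveHealth subtracts one point and updates the widget, or calls OnDeath when one or less remains.
; RespawnPlayer teleports player 0 to StartPoint and resets health to a hardcoded value; AddHealth is an empty stub.
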(event EventBeginPlay
  (bind _maxhealth (Variables|Default|GetmaxHealth))
  ;[1 1 1] Falta comprovación para saber acceder al owner del ac y en caso de ser el jugador crear el widget o no hacerlo si no lo es
  (bind _returnvalue (UserInterface|CreateWidget "/Game/Test/Test_Widgets/W_GamePlayTest.W_GamePlayTest_C"))
  (bind _output_get (Variables|Default|SetW_Gameplay _returnvalue))
  (UserInterface|Viewport|AddtoViewport _output_get 0)
  (bind _output_get_2 (Variables|Default|SetcurrentHealth _maxhealth))
  (Default|SetHealth (Variables|Default|GetW_Gameplay) _output_get_2 _maxhealth))

(fn AddHealth)

(fn RemoveHealth
  (if (<= (Variables|Default|GetcurrentHealth) 1)
    (Default|CallOnDeath)
    (else
      (Variables|Default|SetcurrentHealth (Math|Integer|Max(Integer) 0 (- (Variables|Default|GetcurrentHealth) 1)))
      (Default|SetHealth (Variables|Default|GetW_Gameplay) (Variables|Default|GetcurrentHealth) (Variables|Default|GetmaxHealth)))))

(fn RespawnPlayer
  (Variables|Default|SetcurrentHealth (Math|Integer|Max(Integer) 0 (- (Variables|Default|GetcurrentHealth) 1)))
  (Transformation|Teleport (Game|GetPlayerCharacter 0) (Variables|Default|GetstartPoint) "0, 0, 0")
  (Variables|Default|SetcurrentHealth 3)
  (Default|SetHealth (Variables|Default|GetW_Gameplay) (Variables|Default|GetcurrentHealth) (Variables|Default|GetmaxHealth)))