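; BP_Platform is a platform that rotates its mesh around the yaw axis in response to Switchon and SwitchOff events.
; With CanRotate set, Switchon plays the KeepRotating timeline to drive yaw and SwitchOff reverses it.
; Otherwise, each Switchon lerps the platform a further 90 degrees on a second timeline, with IsRotating blocking retriggers until it finishes, and SwitchOff does nothing.
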(event EventBeginPlay)

(event Collision|EventActorBeginOverlap
  (params (OtherActor :type Actor%20Object%20Reference)))

(event EventTick
  (params (DeltaSeconds :type Float%20%28single-precision%29)))

(event EventSwitchon
  (if (Variables|Default|GetcanRotate)
    (bind _rotation (Timeline|KeepRotating Play)
      (:Update
        (Transformation|SetRelativeRotation (Variables|Default|Getplatform-fortified1) (Math|Rotator|MakeRotator 0.0 0.0 _rotation) false false)))
    (elif (not (Variables|Default|GetisRotating))
      (bind _output_get (Variables|Default|SetcurrentRotation (Variables|Default|GettargetRotation)))
      (Variables|Default|SettargetRotation (+ _output_get 9e+01))
      (bind _newtrack_0 (Timeline|Timeline PlayFromStart)
        (:Update
          (Transformation|SetRelativeRotation (Variables|Default|Getplatform-fortified1) (Math|Rotator|MakeRotator 0.0 0.0 (Math|Float|Lerp (Variables|Default|GetcurrentRotation) (Variables|Default|GettargetRotation) _newtrack_0)) false false)
          (Variables|Default|SetisRotating true))
        (:Finished
          (Variables|Default|SetisRotating false))))))

(event EventSwitchOff
  (if (Variables|Default|GetcanRotate)
    (bind _rotation (Timeline|KeepRotating Reverse)
      (:Update
        (Transformation|SetRelativeRotation (Variables|Default|Getplatform-fortified1) (Math|Rotator|MakeRotator 0.0 0.0 _rotation) false false)))))

(fn ConstructionScript)