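; BP_Box is a test pickup box that the player can carry and throw.
; Each PickObject call toggles the picked flag and prints a debug message.
; Picking teleports the box to a height based on the player character's Z, then attaches it to the pawn's root using KeepRelative rules.
; Releasing detaches it and applies a fixed +X impulse to the Box component.
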(event OnComponentBeginOverlap(Box)
  (params (OverlappedComponent :type Primitive%20Component%20Object%20Reference) (OtherActor :type Actor%20Object%20Reference) (OtherComp :type Primitive%20Component%20Object%20Reference) (OtherBodyIndex :type Integer) (bFromSweep :type Boolean) (SweepResult :type Hit%20Result%20Structure%20%28by%20ref%29)))

(event EventBeginPlay)

(event Collision|EventActorBeginOverlap
  (params (OtherActor :type Actor%20Object%20Reference)))

(event EventTick
  (params (DeltaSeconds :type Float%20%28single-precision%29)))

(event EventPickObject
  (if (not (Variables|Default|GetisBoxPicked))
    (Variables|Default|SetisBoxPicked true)
    (Development|PrintString "Pick Box" true true "(R=1.000000,G=0.000000,B=0.022553,A=1.000000)")
    (CallFunction|TeleportBox)
    (else
      (Variables|Default|SetisBoxPicked false)
      (Development|PrintString "Not Pick Box")
      (CallFunction|LaunchBox))))

(fn ConstructionScript)

(fn TeleportBox
  (Transformation|SetActorLocation (Math|Vector|MakeVector 0.0 0.0 (+ (.z (Transformation|GetActorLocation (Game|GetPlayerCharacter 0))) 275.0)) false true)
  (Transformation|AttachComponentToComponent (Variables|/Script/Engine.Actor|GetRootComponent (Game|Player|GetPlayerPawn 0)) "None" "KeepRelative" "KeepRelative" "KeepRelative" true))

(fn LaunchBox
  (Transformation|DetachFromActor "KeepRelative" "KeepRelative" "KeepRelative")
  (Physics|AddImpulse (Variables|Default|GetBox) "100.000000,0.000000,0.000000" "None" false))